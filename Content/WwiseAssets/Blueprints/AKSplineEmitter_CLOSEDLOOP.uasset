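; AKSplineEmitter_CLOSEDLOOP is a Wwise audio emitter Blueprint, named for a closed-loop spline, with every graph left as a stub.
; BeginPlay and Tick only call the parent, while the emitter update, AK state and player-spawned events are empty.
; Query functions for player distance, inside-spline status, camera rotation and pawn location return zero or false defaults.
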(event Custom|UpdateEmitterLocationProxy)

(event Custom|Update%20Emitter%20Slowly)

(event Custom|Set%20AK%20State)

(event Custom|AKSE_Player_Spawned)

(event EventBeginPlay
  (|CallParentFunction))

(event Collision|EventActorBeginOverlap
  (params (OtherActor :type Actor%20Object%20Reference)))

(event EventTick
  (params (DeltaSeconds :type Float%20%28single-precision%29))
  (|CallParentFunction DeltaSeconds))

(fn ConstructionScript)

(fn GetDistancetoPlayerfromClosestSplinePoint
  (return 0.0))

(fn GetIsInsideSpline
  (return false false))

(fn GetPlayerControllerCameraRotation
  (return ""))

(fn GetControlledPawnLocation
  (return 0 ""))