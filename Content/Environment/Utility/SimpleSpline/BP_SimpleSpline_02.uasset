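; BP_SimpleSpline_02 is a spline utility Blueprint whose function interface covers placing meshes along a spline, though every body here is empty or returns defaults.
; Signatures cover deformable and instanced mesh placement, with meshes sorted or picked by length, index and alternation mode.
; Further stubs cover alignment tests, tinting, debug colours and stats, and attaching actors to spline points.
; The construction script and events contain no logic.
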(event Custom|Add%20Chain%20Actor)

(event Custom|Add%20Start%20Actor)

(event EventBeginPlay)

(event Collision|EventActorBeginOverlap
  (params (OtherActor :type Actor%20Object%20Reference)))

(event EventTick
  (params (DeltaSeconds :type Float%20%28single-precision%29)))

(fn ConstructionScript)

(fn TintMesh
  (params (Mesh%20Component :type Static%20Mesh%20Component%20Object%20Reference%20%28by%20ref%29) (Color :type Linear%20Color%20Structure%20%28by%20ref%29)))

(fn AddDebugStats
  (params (Debug%20Enabled :type Boolean) (Spline :type Spline%20Component%20Object%20Reference%20%28by%20ref%29) (Start%20Distance :type Float%20%28single-precision%29) (End%20Distance :type Float%20%28single-precision%29) (Mesh%20Lenght :type Float%20%28single-precision%29) (Mesh%20Type :type String) (Mesh%20Name :type String) (Text%20Color :type Linear%20Color%20Structure) (Mesh%20Number :type Integer)))

(fn UpdateAtachment
  (params (Actor :type Actor%20Object%20Reference%20%28by%20ref%29) (Spline%20Point%20Index :type Integer)))

(fn GetColor
  (params (Color%20Array :type Array%20of%20Linear%20Color%20Structures) (Index :type Integer))
  (return ""))

(fn SetDebugColor
  (params (Mesh :type Spline%20Mesh%20Component%20Object%20Reference) (Debug%20Enabled :type Boolean) (Linear%20Color :type Linear%20Color%20Structure)))

(fn AddInstancedMeshtoSpline
  (params (Spline :type Spline%20Component%20Object%20Reference%20%28by%20ref%29) (Mesh :type Static%20Mesh%20Object%20Reference%20%28by%20ref%29) (Distance :type Float%20%28single-precision%29) (Offset :type Float%20%28single-precision%29) (Reverse :type Boolean) (Scale :type Float%20%28single-precision%29) (Rotation :type Rotator))
  (return 0))

(fn AddDeformableMeshtoSpline
  (params (Forward%20Axis :type ESplineMeshAxis%20Enum%20%28by%20ref%29 :default "X") (Mesh :type Static%20Mesh%20Object%20Reference%20%28by%20ref%29) (Spline :type Spline%20Component%20Object%20Reference%20%28by%20ref%29) (Mesh%20Scale :type Float%20%28single-precision%29) (Start%20Distance :type Float%20%28single-precision%29%20%28by%20ref%29) (Start%20Offset :type Float%20%28single-precision%29) (End%20Distance :type Float%20%28single-precision%29%20%28by%20ref%29) (Clamp%20Tangent :type Boolean) (Clamp%20Tangent%20Size :type Float%20%28single-precision%29) (is%20Debug%20Enabled :type Boolean) (Debug%20Color :type Linear%20Color%20Structure))
  (return 0))

(fn GetMaximumLenght
  (params (Struct%20Array :type Array%20of%20Length%20Mesh%20Array%20Structures))
  (return 0.0))

(fn SelectStructArray
  (params (Direction%20Vector :type Vector%20%28by%20ref%29))
  (return 0 "X" ""))

(fn TestAlignmentFactor
  (params (Test%20Vector :type Vector%20%28by%20ref%29) (Alignment%20Factor%20Threshold :type Float%20%28single-precision%29))
  (return false))

(fn MakeSortedSrtructArray
  (params (Spline%20Meshes :type Array%20of%20Static%20Mesh%20Object%20References) (Forward%20Axis :type ESplineMeshAxis%20Enum%20%28by%20ref%29 :default "X"))
  (return 0))

(fn SortbyLength
  (params (Mesh%20Array :type Array%20of%20Static%20Mesh%20Object%20References) (Forward%20Axis :type ESplineMeshAxis%20Enum%20%28by%20ref%29 :default "X")))

(fn GetRandomMeshbyIndex
  (params (Index :type Integer) (Mesh%20Array :type Array%20of%20Length%20Mesh%20Array%20Structures) (Alternation%20Mode :type Boolean) (Counter :type Integer))
  (return 0 0.0))

(fn GetRandomMeshbyLength
  (params (Length :type Float%20%28single-precision%29) (Mesh%20Scale%20Multiplier :type Float%20%28single-precision%29) (Mesh%20Array :type Array%20of%20Length%20Mesh%20Array%20Structures) (Alternation%20Mode :type Boolean) (Counter :type Integer))
  (return 0 0.0))

(fn GetMeshArraybyLength
  (params (Mesh%20Array :type Array%20of%20Static%20Mesh%20Object%20References) (Forward%20Axis :type ESplineMeshAxis%20Enum :default "X") (Length :type Float%20%28single-precision%29))
  (return 0))